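; Farm tile actor where the player plants a seed, watches it grow and harvests it; only wheat is implemented.
; PlantSeed takes the seed from the player's inventory and counter, then swaps runtime-added meshes through three growth stages.
; The GrowTime macro paces each stage with a looping one-second Delay countdown shown on Text3D.
; Activate calls Harvest, which, once fully grown, spawns wheat, seed and pickup actors and frees the tile.
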(event Custom|PlantWheat
  (params (charRef :type Third%20Person%20Character%20Object%20Reference))
  (bind _relativetransformlocation (Variables|Default|GetRelativeTransformLocation))
  (bind _inventoryref (Variables|/Game/ThirdPersonBP/Blueprints/ThirdPersonCharacter.ThirdPersonCharacter_C|GetInventoryRef charRef))
  (bind _asthird_person_character (Utilities|Casting|CastToThirdPersonCharacter (Game|GetPlayerCharacter 0)))
  (Default|RemoveItematIndex _inventoryref (.Index (Default|FindItemIWant _inventoryref "/Game/Inventory/Blueprints/ItemClasses/Seed_imsi.Seed_imsi_C")) 1)
  (Math|Integer|DecrementInt (Variables|/Game/ThirdPersonBP/Blueprints/ThirdPersonCharacter.ThirdPersonCharacter_C|GetAmountOfWheatSeed _asthird_person_character)
    (:%20%20
      (bind _returnvalue (AddComponent|AddStaticMeshComponent false (Math|Transform|MakeTransform _relativetransformlocation "0, 0, 0" "1,1,1")))
      (Utilities|GrowTime (Variables|Default|GetWheatGrowTime)
        (:Out
          (Components|DestroyComponent _returnvalue)
          (bind _returnvalue_2 (AddComponent|AddStaticMeshComponent false (Math|Transform|MakeTransform _relativetransformlocation "0, 0, 0" "1,1,1")))
          (Utilities|GrowTime (Variables|Default|GetWheatGrowTime)
            (:Out
              (Components|DestroyComponent _returnvalue_2)
              (bind _returnvalue_3 (AddComponent|AddStaticMeshComponent false (Math|Transform|MakeTransform _relativetransformlocation "0, 0, 0" "1,1,1")))
              (Variables|Default|SetCurrentMesh _returnvalue_3)
              (Variables|Default|SetFullyGrown? true)
              (Variables|Default|SetWhatCanBeHarvested "Wheat"))))))))

(event EventBeginPlay
  (Class|Text3DComponent|SetText (Variables|Default|GetText3D) (Variables|Default|GetValue)))

(event Collision|EventActorBeginOverlap
  (params (OtherActor :type Actor%20Object%20Reference)))

(event EventTick
  (params (DeltaSeconds :type Float%20%28single-precision%29)))

(event EventPlantSeed
  (params (charRef :type Third%20Person%20Character%20Object%20Reference))
  (if (not (Variables|Default|GetIsSomethingPlanted?))
    (bind _asthird_person_character (Utilities|Casting|CastToThirdPersonCharacter (Game|GetPlayerCharacter 0)))
    (switch int (Variables|/Game/ThirdPersonBP/Blueprints/ThirdPersonCharacter.ThirdPersonCharacter_C|Getseed _asthird_person_character)
      (:0
        (CallFunction|PlantWheat charRef)
        (Variables|Default|SetIsSomethingPlanted? true)))))

(event EventActivate
  (CallFunction|Harvest))

(fn ConstructionScript)

(fn Harvest
  (bind _text3d (Variables|Default|GetText3D))
  (bind _returnvalue (Transformation|GetWorldLocation _text3d))
  (bind _returnvalue_2 (Math|Conversions|ToTransform(Vector) _returnvalue))
  (if (Variables|Default|GetFullyGrown?)
    (Components|DestroyComponent (Variables|Default|GetCurrentMesh))
    (switch string (Variables|Default|GetWhatCanBeHarvested)
      (:Default
        _)
      (:Wheat
        (Game|SpawnActorfromClass "/Game/Inventory/Blueprints/ItemClasses/BP_PickupActor.BP_PickupActor_C" (Math|Conversions|ToTransform(Vector) (- _returnvalue "0, 0,200.000000")) "Undefined" 0 "/Game/Inventory/Blueprints/ItemClasses/Seed_imsi.Seed_imsi_C" 1 0)
        ;[1 1 1] WheatSpawn
        (Game|SpawnActorfromClass "/Game/Planting/BP_Wheat.BP_Wheat_C" _returnvalue_2 "Undefined" 0 0)
        ;[1 1 1] SeedSpawn
        (Game|SpawnActorfromClass "/Game/Planting/BP_Wheat_Seed.BP_Wheat_Seed_C" _returnvalue_2 "Undefined" 0 0)))
    (Variables|Default|SetFullyGrown? false)
    (Variables|Default|SetCurrentMesh 0)
    (Variables|Default|SetIsSomethingPlanted? false)))