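; Interactable chest actor that opens a storage inventory for the player and freezes their movement while it is open.
; An overlap range toggles a prompt text and registers the chest as the character's nearby chest.
; On interact, a DoOnce guard lazily spawns a Bp_Storage actor, builds its slot widgets and shows it beside the refreshed inventory.
; Closing hides storage, restores walking and resets the guard.
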(event OnComponentBeginOverlap(InteractionRange)
  (params (OverlappedComponent :type Primitive%20Component%20Object%20Reference) (OtherActor :type Actor%20Object%20Reference) (OtherComp :type Primitive%20Component%20Object%20Reference) (OtherBodyIndex :type Integer) (bFromSweep :type Boolean) (SweepResult :type Hit%20Result%20Structure%20%28by%20ref%29))
  (bind _asthird_person_character (Utilities|Casting|CastToThirdPersonCharacter OtherActor))
  (Rendering|SetVisibility (Variables|Default|GetChestText) true false)
  (Variables|/Game/ThirdPersonBP/Blueprints/ThirdPersonCharacter.ThirdPersonCharacter_C|SetNearByChest _asthird_person_character self))

(event OnComponentEndOverlap(InteractionRange)
  (params (OverlappedComponent :type Primitive%20Component%20Object%20Reference) (OtherActor :type Actor%20Object%20Reference) (OtherComp :type Primitive%20Component%20Object%20Reference) (OtherBodyIndex :type Integer))
  (bind _asthird_person_character (Utilities|Casting|CastToThirdPersonCharacter OtherActor))
  (Rendering|SetVisibility (Variables|Default|GetChestText) false false)
  (Variables|/Game/ThirdPersonBP/Blueprints/ThirdPersonCharacter.ThirdPersonCharacter_C|SetNearByChest _asthird_person_character 0))

(event Custom|OnStorageClosed
  (Default|HideStorage (Variables|Default|GetStorageActor))
  (Pawn|Components|CharacterMovement|SetMovementMode (Variables|/Script/Engine.Character|GetCharacterMovement (Variables|Default|GetCharRef)) "MOVE_Walking" 0)
  (if (Variables|/Game/Inventory/Blueprints/BP_Inventory.BP_Inventory_C|GetisVisible? (Variables|/Game/ThirdPersonBP/Blueprints/ThirdPersonCharacter.ThirdPersonCharacter_C|GetInventoryRef (Variables|Default|GetCharRef)))
    (Default|HideInventory (Variables|/Game/ThirdPersonBP/Blueprints/ThirdPersonCharacter.ThirdPersonCharacter_C|GetInventoryRef (Variables|Default|GetCharRef)))
    (Default|ShowInventory (Variables|/Game/ThirdPersonBP/Blueprints/ThirdPersonCharacter.ThirdPersonCharacter_C|GetInventoryRef (Variables|Default|GetCharRef)))
    (Utilities|FlowControl|DoOnce false) ; enters at Reset
    (else
      (Utilities|FlowControl|DoOnce false) ; enters at Reset
    )))

(event Custom|OnInteract
  (params (CharRef :type Third%20Person%20Character%20Object%20Reference))
  (Utilities|FlowControl|DoOnce false
    (:Completed
      (Variables|Default|SetCharRef CharRef)
      (Utilities|IsValid (Variables|Default|GetStorageActor)
        (:Is%20Valid
          _)
        (:Is%20Not%20Valid
          (bind _returnvalue (Game|SpawnActorfromClass "/Game/Inventory/Blueprints/Bp_Storage.Bp_Storage_C" (Math|Transform|MakeTransform "0, 0, 0" "0, 0, 0" "1,1,1") "AlwaysSpawn" 0 (Variables|Default|GetAmountOfSlots) (Variables|Default|GetCharRef) (Variables|Default|GetSlotsPerRow) self 0))
          (Variables|Default|SetStorageActor _returnvalue)))
      (Default|GenerateSlotWidgets (Variables|/Game/Inventory/Blueprints/Bp_Storage.Bp_Storage_C|GetStorageWidget (Variables|Default|GetStorageActor)) (Variables|Default|GetStorageActor))
      (Default|ShowStorage (Variables|Default|GetStorageActor))
      (Default|HideInventory (Variables|/Game/ThirdPersonBP/Blueprints/ThirdPersonCharacter.ThirdPersonCharacter_C|GetInventoryRef (Variables|Default|GetCharRef)))
      (Default|ShowInventory (Variables|/Game/ThirdPersonBP/Blueprints/ThirdPersonCharacter.ThirdPersonCharacter_C|GetInventoryRef (Variables|Default|GetCharRef)))
      (Pawn|Components|CharacterMovement|DisableMovement (Variables|/Script/Engine.Character|GetCharacterMovement (Variables|Default|GetCharRef)))
      (Components|Movement|StopMovementImmediately (Variables|/Script/Engine.Character|GetCharacterMovement (Variables|Default|GetCharRef))))))

(event EventBeginPlay)

(event Collision|EventActorBeginOverlap
  (params (OtherActor :type Actor%20Object%20Reference)))

(event EventTick
  (params (DeltaSeconds :type Float%20%28single-precision%29)))

(fn ConstructionScript)