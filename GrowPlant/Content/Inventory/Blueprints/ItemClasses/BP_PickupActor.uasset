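; BP_PickupActor is a world pickup that adds an item to the player's inventory when touched.
; When the Sphere overlaps a ThirdPersonCharacter with a valid InventoryRef, it calls AddItem with its ItemToAdd class and Amount.
; On success it keeps any leftover Rest as its new Amount, or destroys itself when nothing remains, allowing partial pickups.
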(event OnComponentBeginOverlap(Sphere)
  (params (OverlappedComponent :type Primitive%20Component%20Object%20Reference) (OtherActor :type Actor%20Object%20Reference) (OtherComp :type Primitive%20Component%20Object%20Reference) (OtherBodyIndex :type Integer) (bFromSweep :type Boolean) (SweepResult :type Hit%20Result%20Structure%20%28by%20ref%29))
  (bind _asthird_person_character (Utilities|Casting|CastToThirdPersonCharacter OtherActor))
  (Utilities|IsValid (Variables|/Game/ThirdPersonBP/Blueprints/ThirdPersonCharacter.ThirdPersonCharacter_C|GetInventoryRef _asthird_person_character)
    (:Is%20Valid
      (bind (_success_ _rest) (Default|AddItem (Variables|/Game/ThirdPersonBP/Blueprints/ThirdPersonCharacter.ThirdPersonCharacter_C|GetInventoryRef _asthird_person_character) (Variables|Default|GetItemToAdd) (Variables|Default|GetAmount)))
      (if _success_
        (if (> _rest 0)
          (Variables|Default|SetAmount _rest)
          (else
            (Actor|DestroyActor)))))))

(event EventBeginPlay)

(event Collision|EventActorBeginOverlap
  (params (OtherActor :type Actor%20Object%20Reference)))

(event EventTick
  (params (DeltaSeconds :type Float%20%28single-precision%29)))

(fn ConstructionScript)