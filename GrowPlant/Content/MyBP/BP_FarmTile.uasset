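; BP_FarmTile is a farm tile that plants a crop from the player character's selected seed and grows it over time, with wheat the only crop handled.
; PlantSeed skips occupied tiles, then PlantWheat swaps dynamically added static mesh components through three growth stages.
; The GrowTime macro separates stages with a one-second Delay loop, showing the countdown on the tile's Text3D.
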(event Custom|PlantWheat
  (bind _relativetransformlocation (Variables|Default|GetRelativeTransformLocation))
  (bind _returnvalue (AddComponent|AddStaticMeshComponent false (Math|Transform|MakeTransform _relativetransformlocation "0, 0, 0" "1,1,1")))
  (Utilities|GrowTime (Variables|Default|GetWheatGrowTime)
    (:Out
      (Components|DestroyComponent _returnvalue)
      (bind _returnvalue_2 (AddComponent|AddStaticMeshComponent false (Math|Transform|MakeTransform _relativetransformlocation "0, 0, 0" "1,1,1")))
      (Utilities|GrowTime (Variables|Default|GetWheatGrowTime)
        (:Out
          (Components|DestroyComponent _returnvalue_2)
          (AddComponent|AddStaticMeshComponent false (Math|Transform|MakeTransform _relativetransformlocation "0, 0, 0" "1,1,1")))))))

(event EventBeginPlay
  (Class|Text3DComponent|SetText (Variables|Default|GetText3D) (Variables|Default|GetValue)))

(event Collision|EventActorBeginOverlap
  (params (OtherActor :type Actor%20Object%20Reference)))

(event EventTick
  (params (DeltaSeconds :type Float%20%28single-precision%29)))

(event EventPlantSeed
  (if (not (Variables|Default|GetIsSomethingPlanted?))
    (bind _asthird_person_character (Utilities|Casting|CastToThirdPersonCharacter (Game|GetPlayerCharacter 0)))
    (switch int (Variables|/Game/ThirdPersonBP/Blueprints/ThirdPersonCharacter.ThirdPersonCharacter_C|Getseed _asthird_person_character)
      (:0
        (CallFunction|PlantWheat)
        (Variables|Default|SetIsSomethingPlanted? true)))))

(fn ConstructionScript)