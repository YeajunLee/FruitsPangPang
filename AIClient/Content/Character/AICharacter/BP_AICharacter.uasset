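; BP_AICharacter is an AI-controlled character Blueprint that can spawn a bomb in its hand socket.
; Tick stores horizontal movement speed in GroundSpeedAI by zeroing the vertical velocity before taking its length.
; ThrowAIBP spawns a Bomb at the mesh's BombSocket, keeps it in Projectile0 and attaches it to that socket.
; Despite its name, the function applies no launch or release, and nothing in this file calls it.
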(event EventBeginPlay)

(event Collision|EventActorBeginOverlap
  (params (OtherActor :type Actor%20Object%20Reference)))

(event EventTick
  (params (DeltaSeconds :type Float%20%28single-precision%29))
  (Variables|Default|SetGroundSpeed_AI (Math|Vector|VectorLength (* (Variables|/Script/Engine.MovementComponent|GetVelocity (Variables|Character|GetCharacterMovement)) "1.000000,1.000000, 0"))))

(fn ConstructionScript)

(fn ThrowAIBP
  (bind _returnvalue (Game|SpawnActorfromClass "/Game/Assets/Fruits/tomato/Bomb.Bomb_C" (Transformation|GetSocketTransform (Variables|Character|GetMesh) "BombSocket" "RTS_World") "Undefined" 0 0))
  (bind _output_get (Variables|Default|SetProjectile_0 _returnvalue))
  (Transformation|AttachComponentToComponent _output_get (Variables|Character|GetMesh) "BombSocket" "KeepWorld" "KeepWorld" "KeepRelative" true))