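; BP_MatchHelper is an NPC helper Blueprint, filed under MatchingNpc, that shows a speech bubble when the player character comes near.
; Begin and end overlap events on MBoxCollision filter for MyCharacter, then show or hide the speech bubble component (말풍선) and two TextRender components.
; Visibility changes do not propagate to children, and BeginPlay, Tick and the construction script are empty.
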(event OnComponentBeginOverlap(mBoxCollision)
  (params (OverlappedComponent :type Primitive%20Component%20Object%20Reference) (OtherActor :type Actor%20Object%20Reference) (OtherComp :type Primitive%20Component%20Object%20Reference) (OtherBodyIndex :type Integer) (bFromSweep :type Boolean) (SweepResult :type Hit%20Result%20Structure%20%28by%20ref%29))
  (Utilities|Casting|CastToMyCharacter OtherActor)
  (Rendering|SetVisibility (Variables|Default|Get말풍선) true false)
  (Rendering|SetVisibility (Variables|Default|GetTextRender) true false)
  (Rendering|SetVisibility (Variables|Default|GetTextRender1) true false))

(event OnComponentEndOverlap(mBoxCollision)
  (params (OverlappedComponent :type Primitive%20Component%20Object%20Reference) (OtherActor :type Actor%20Object%20Reference) (OtherComp :type Primitive%20Component%20Object%20Reference) (OtherBodyIndex :type Integer))
  (Utilities|Casting|CastToMyCharacter OtherActor)
  (Rendering|SetVisibility (Variables|Default|Get말풍선) false false)
  (Rendering|SetVisibility (Variables|Default|GetTextRender) false false)
  (Rendering|SetVisibility (Variables|Default|GetTextRender1) false false))

(event EventBeginPlay)

(event Collision|EventActorBeginOverlap
  (params (OtherActor :type Actor%20Object%20Reference)))

(event EventTick
  (params (DeltaSeconds :type Float%20%28single-precision%29)))

(fn ConstructionScript)