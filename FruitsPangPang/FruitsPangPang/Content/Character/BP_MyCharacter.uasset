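; Character Blueprint that reacts to fruit projectile hits and sets up its POI component's enemy images.
; BeginPlay blanks the second and third enemy images, plus the first for player 0; any key press forwards to AnyKeyPressed.
; Capsule hits by a Projectile write to FruitArr by fruit type, set IsHit and pulse HitbyFruit briefly for hit animation.
; Footprint events are empty; the tomato footprint spawning logic is disconnected and never runs.
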(event OnComponentHit(CapsuleComponent)
  (params (HitComponent :type Primitive%20Component%20Object%20Reference) (OtherActor :type Actor%20Object%20Reference) (OtherComp :type Primitive%20Component%20Object%20Reference) (NormalImpulse :type Vector :default "0, 0, 0") (Hit :type Hit%20Result%20Structure%20%28by%20ref%29))
  ;[1 1 1] Hit 애니메이션을 위한 과일과 충돌처리
  (bind _asprojectile (Utilities|Casting|CastToProjectile OtherActor))
  (Utilities|Array|SetArrayElem (Variables|Default|GetFruitArr) (Variables|/Script/FruitsPangPang.Projectile|Get_fType _asprojectile) 0)
  (if true
    (Variables|Default|Setis%20Hit? true)
    (Variables|Default|SetbHitbyFruit true)
    (Utilities|FlowControl|Delay 0.3)
    (Variables|Default|SetbHitbyFruit false)
    (else
      (Variables|Default|Setis%20Hit? false)
      (Variables|Default|SetbHitbyFruit false))))

(event Custom|SpawnFootprintR
  ;[1 1 1] Spawn Footprint
)

(event Custom|SpawnFootpirintL
  ;[1 1 1] Spawn Footprint
)

(event EventBeginPlay
  (Variables|/Script/FruitsPangPang.PointOfInterestComponent|SetEnemy2Image (Variables|Default|GetPOIcomponent) "/Game/MiniMap/NothingIMG.NothingIMG")
  (Variables|/Script/FruitsPangPang.PointOfInterestComponent|SetEnemy3Image (Variables|Default|GetPOIcomponent) "/Game/MiniMap/NothingIMG.NothingIMG")
  (if (== (Game|GetPlayerCharacter 0) self)
    (Variables|/Script/FruitsPangPang.PointOfInterestComponent|SetEnemy1Image (Variables|Default|GetPOIcomponent) "/Game/MiniMap/NothingIMG.NothingIMG")))

(event Input|KeyboardEvents|AnyKey
  (params (Key :type Key%20Structure :default "None"))
  (:Pressed
    (Class|MyCharacter|AnyKeyPressed Key)))

(fn ConstructionScript)