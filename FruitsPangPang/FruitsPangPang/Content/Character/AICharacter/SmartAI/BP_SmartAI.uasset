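; Smart AI character that jumps over obstacles while moving and reacts to fruit projectile hits.
; On Tick, above a speed threshold, it traces a short line forward, ignoring itself and listed actor classes; a hit triggers a jump, then NavWalking after a delay.
; Capsule hits from Projectiles write to FruitArr at the fruit-type index and set hit flags for animation, with HitbyFruit clearing shortly after.
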(event OnComponentHit(CapsuleComponent)
  (params (HitComponent :type Primitive%20Component%20Object%20Reference) (OtherActor :type Actor%20Object%20Reference) (OtherComp :type Primitive%20Component%20Object%20Reference) (NormalImpulse :type Vector :default "0, 0, 0") (Hit :type Hit%20Result%20Structure%20%28by%20ref%29))
  ;[1 1 1] Hit 애니메이션을 위한 과일과 충돌처리
  (bind _asprojectile (Utilities|Casting|CastToProjectile OtherActor))
  (Utilities|Array|SetArrayElem (Variables|Default|GetFruitArr) (Variables|/Script/FruitsPangPang.Projectile|Get_fType _asprojectile) 0)
  (if true
    (Variables|Default|Setis%20Hit? true)
    (Variables|Default|SetbHitbyFruit true)
    (Utilities|FlowControl|Delay 0.3)
    (Variables|Default|SetbHitbyFruit false)
    (else
      (Variables|Default|Setis%20Hit? false)
      (Variables|Default|SetbHitbyFruit false))))

(event EventBeginPlay)

(event Collision|EventActorBeginOverlap
  (params (OtherActor :type Actor%20Object%20Reference)))

(event EventTick
  (params (DeltaSeconds :type Float%20%28single-precision%29))
  (bind _returnvalue (Transformation|GetActorLocation))
  (if (>= (Math|Vector|VectorLength (Transformation|GetVelocity)) 1e+02)
    (for _array_element (Variables|Default|GetIgnore%20Classes)
      (bind _outactors (Actor|GetAllActorsOfClass _array_element))
      (for _array_element_2 _outactors
        (Utilities|Array|Add (Variables|Default|GetOut%20Actors) _array_element_2)))
    (Utilities|Array|Add (Variables|Default|GetOut%20Actors) self)
    (bind _returnvalue_2 (Collision|LineTraceForObjects _returnvalue (+ _returnvalue (* (Transformation|GetActorForwardVector) 2.5e+02)) (Variables|Default|GetObject%20Types) false (Variables|Default|GetOut%20Actors) "ForOneFrame"))
    (if _returnvalue_2
      (Character|Jump)
      (Utilities|FlowControl|Delay 0.2)
      (Pawn|Components|CharacterMovement|SetMovementMode (Variables|Character|GetCharacterMovement) "MOVE_NavWalking" 0))))

(fn ConstructionScript)