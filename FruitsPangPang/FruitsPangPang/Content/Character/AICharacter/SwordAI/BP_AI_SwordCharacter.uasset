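; Sword AI character that automatically jumps when an obstacle appears ahead while it moves.
; On Tick, above a minimum speed, it traces forward for configured object types, ignoring itself and all actors of the IgnoreClasses.
; A hit triggers Jump, then a short delay switches movement to NavWalking.
; The ignore list is appended every Tick without clearing, and debug leftovers include trace drawing and a BeginPlay print.
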(event EventBeginPlay
  (Development|PrintString "Hello"))

(event Collision|EventActorBeginOverlap
  (params (OtherActor :type Actor%20Object%20Reference)))

(event EventTick
  (params (DeltaSeconds :type Float%20%28single-precision%29))
  (bind _returnvalue (Transformation|GetActorLocation))
  (Utilities|FlowControl|Sequence
    (:then_1
      (if (>= (Math|Vector|VectorLength (Transformation|GetVelocity)) 1e+02)
        (for _array_element (Variables|Default|GetIgnore%20Classes)
          (bind _outactors (Actor|GetAllActorsOfClass _array_element))
          (for _array_element_2 _outactors
            (Utilities|Array|Add (Variables|Default|GetOut%20Actors) _array_element_2)))
        (Utilities|Array|Add (Variables|Default|GetOut%20Actors) self)
        (bind _returnvalue_2 (Collision|LineTraceForObjects _returnvalue (+ _returnvalue (* (Transformation|GetActorForwardVector) 2.5e+02)) (Variables|Default|GetObject%20Types) false (Variables|Default|GetOut%20Actors) "ForOneFrame"))
        (if _returnvalue_2
          (Character|Jump)
          (Utilities|FlowControl|Delay 0.2)
          (Pawn|Components|CharacterMovement|SetMovementMode (Variables|Character|GetCharacterMovement) "MOVE_NavWalking" 0))))))

(fn ConstructionScript)