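; Spoon and cherry fountain map object with a FountainOn switch that turns its water effects on or off.
; The construction script sets the fountain and ripple-flatten values in two Material Parameter Collections and shows or hides the particle system.
; Tick re-applies only the ripple-flatten value every frame, so the fountain parameter and particle visibility change only when construction runs.
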(event EventBeginPlay)

(event Collision|EventActorBeginOverlap
  (params (OtherActor :type Actor%20Object%20Reference)))

(event EventTick
  (params (DeltaSeconds :type Float%20%28single-precision%29))
  (if (Variables|Default|GetFountainOn)
    (Rendering|Material|SetScalarParameterValue "/Game/Maps/Fountain/RainyWeather/NewMaterialParameterCollection.NewMaterialParameterCollection" "Ripple Flatten" 0.0 :!class /Script/Engine.KismetMaterialLibrary)
    (else
      (Rendering|Material|SetScalarParameterValue "/Game/Maps/Fountain/RainyWeather/NewMaterialParameterCollection.NewMaterialParameterCollection" "Ripple Flatten" 1.0 :!class /Script/Engine.KismetMaterialLibrary))))

(fn ConstructionScript
  (bind _particlesystem (Variables|Default|GetParticleSystem))
  (if (Variables|Default|GetFountainOn)
    (Rendering|Material|SetScalarParameterValue "/Game/Maps/Fountain/RainyWeather/NewMaterialParameterCollection.NewMaterialParameterCollection" "Ripple Flatten" 0.0 :!class /Script/Engine.KismetMaterialLibrary)
    (Rendering|Material|SetScalarParameterValue "/Game/Maps/Fountain/MPC_Fountain.MPC_Fountain" "Fountain" 1.0 :!class /Script/Engine.KismetMaterialLibrary)
    (Rendering|SetVisibility _particlesystem true false)
    (else
      (Rendering|Material|SetScalarParameterValue "/Game/Maps/Fountain/RainyWeather/NewMaterialParameterCollection.NewMaterialParameterCollection" "Ripple Flatten" 1.0 :!class /Script/Engine.KismetMaterialLibrary)
      (Rendering|Material|SetScalarParameterValue "/Game/Maps/Fountain/MPC_Fountain.MPC_Fountain" "Fountain" 0.0 :!class /Script/Engine.KismetMaterialLibrary)
      (Rendering|SetVisibility _particlesystem false false))))