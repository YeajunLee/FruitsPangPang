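; Destructible watermelon actor that shatters when it hits something and damages the actor it struck.
; Each component hit applies destructible damage at an arrow component, pushing along the arrow's forward vector.
; A DoOnce gate limits the C++ damage call on the other actor, the particle burst and the sound to the first hit, then the actor destroys itself after a short delay.
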(event OnComponentHit(Destructible)
  (params (HitComponent :type Primitive%20Component%20Object%20Reference) (OtherActor :type Actor%20Object%20Reference) (OtherComp :type Primitive%20Component%20Object%20Reference) (NormalImpulse :type Vector :default "0, 0, 0") (Hit :type Hit%20Result%20Structure%20%28by%20ref%29))
  (bind _arrow (Variables|Default|GetArrow))
  (Class|DestructibleComponent|ApplyDamage (Variables|Default|GetDestructible) 1e+01 (Transformation|GetWorldLocation _arrow) (Math|Vector|GetForwardVector _arrow) 1e+01)
  (Utilities|FlowControl|DoOnce false
    (:Completed
      (Class|Projectile|ApplyDamageCPP OtherActor)
      (Effects|SpawnEmitteratLocation "/Game/Assets/Fruits/Watermelon/P_Watermelon.P_Watermelon" (Transformation|GetWorldLocation (Variables|Default|GetDestructible)) "0, 0, 0" "0.300000,0.300000,0.300000")
      (Audio|PlaySoundatLocation "/Game/Assets/Sounds/Watermelon_Sound.Watermelon_Sound" (Transformation|GetActorLocation) "0, 0, 0" 1.0 1.0 0.0 0 0 0)
      (Utilities|FlowControl|Delay 3.0)
      (Actor|DestroyActor))))

(event EventBeginPlay)

(event Collision|EventActorBeginOverlap
  (params (OtherActor :type Actor%20Object%20Reference)))

(event EventTick
  (params (DeltaSeconds :type Float%20%28single-precision%29)))

(fn ConstructionScript)